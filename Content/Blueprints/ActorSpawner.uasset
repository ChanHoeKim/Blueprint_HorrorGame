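; Spawner actor for the item collection objective, scattering CollectObject pickups inside its Box volume.
; BeginPlay stores and prints the level name, then binds spawning to the StartCollectObject actor's OnClick dispatcher, which triggers a loop placing pickups at random points in the box.
; Tick polls BP_Player's ItemAccount and, once it reaches the required count, calls AllCollect and disables its own tick.
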(event `self.ReceiveBeginPlay`
  (bind _returnvalue (`GameplayStatics.GetCurrentLevelName` true))
  (bind _output_get (set `self.NowLevel` _returnvalue))
  (`KismetSystemLibrary.PrintString` _output_get)
  (bind _returnvalue_2 (`GameplayStatics.GetActorOfClass` "/Game/Blueprints/StartWidget/StartCollectObject.StartCollectObject_C"))
  (add `/Game/Blueprints/StartWidget/StartCollectObject.Onclick` _returnvalue_2 (delegate `SpawnCollectObject`)))

(event `SpawnCollectObject`
  (bind _box (`self.Box`))
  (bind (_returnvalue_x _returnvalue_y _returnvalue_z) (`KismetMathLibrary.BreakVector` (`KismetMathLibrary.RandomPointInBoundingBox` (`SceneComponent.K2_GetComponentLocation` _box) (`BoxComponent.GetScaledBoxExtent` _box))))
  (`self.SetOwner` null)
  (for _ (range 61)
    (`|SpawnActorFromClass` "/Game/Blueprints/CollectObject.CollectObject_C" (`KismetMathLibrary.MakeTransform` (`KismetMathLibrary.MakeVector` _returnvalue_x _returnvalue_y _returnvalue_z)) "AdjustIfPossibleButAlwaysSpawn" "MultiplyWithRoot" null null)))

(event `self.ReceiveTick`
  (params (DeltaSeconds :type "Float (single-precision)"))
  (bind _asbp_player (cast `/Game/Blueprints/BP_Player` (`GameplayStatics.GetPlayerCharacter` 0)))
  (if (>= (`/Game/Blueprints/BP_Player.ItemAccount` _asbp_player) 3.0)
    (`self.AllCollect`)
    (`self.SetActorTickEnabled` false)))

(fn `UserConstructionScript`)