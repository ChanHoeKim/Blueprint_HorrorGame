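; Level exit door for the Backrooms that opens once an ActorSpawner signals that everything has been collected.
; On BeginPlay it binds OpenDoor to that event, which blends the view to the door's camera and swings the mesh 90 degrees with a timeline.
; After a delay the view blends back to the player.
; Once open, a player-tagged actor entering the trigger box loads the Demo level.
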(event `self.ReceiveBeginPlay`
  (bind _outactors (`GameplayStatics.GetAllActorsOfClass` "/Game/Blueprints/ActorSpawner.ActorSpawner_C"))
  (add `/Game/Blueprints/ActorSpawner.AllCollect` _outactors (delegate `OpenDoor`)))

(event `OpenDoor`
  (bind _camera (`self.Camera`))
  (bind (_relativelocation_x _relativelocation_y _relativelocation_z) (`KismetMathLibrary.BreakVector` (`SceneComponent.RelativeLocation` _camera)))
  (set `self.isOpenDoor` true)
  (`PlayerController.SetViewTargetWithBlend` (`GameplayStatics.GetPlayerController` 0) (`ActorComponent.GetOwner` (`self.Camera`)) 0.325 "VTBlend_Linear" 0.0 false)
  (`Timeline|타임라인`
    (:`Update`
      (`SceneComponent.K2_SetRelativeLocation` _camera (`KismetMathLibrary.MakeVector` _relativelocation_x _relativelocation_y _relativelocation_z) false false)
      (bind (_direction _doortimer) (`Timeline|DoorTime`)
        (:`Update`
          (`SceneComponent.K2_SetRelativeRotation` (`self.SM_Door`) (`KismetMathLibrary.MakeRotator` 0.0 0.0 (* _doortimer 90.0)) false false)
          (bind _asbp_player (cast `/Game/Blueprints/BP_Player` (`GameplayStatics.GetPlayerCharacter` 0)))
          (`KismetSystemLibrary.Delay` 3.0)
          (`PlayerController.SetViewTargetWithBlend` (`GameplayStatics.GetPlayerController` 0) _asbp_player 0.325 "VTBlend_Linear" 0.0 false)
          (`Timeline|타임라인_0`
            (:`Update`
              (bind _firstpersoncamera (`/Game/Blueprints/BP_Player.FirstPersonCamera` _asbp_player))
              (bind (_relativelocation_x_2 _relativelocation_y_2 _relativelocation_z_2) (`KismetMathLibrary.BreakVector` (`SceneComponent.RelativeLocation` _firstpersoncamera)))
              (`SceneComponent.K2_SetRelativeLocation` _firstpersoncamera (`KismetMathLibrary.MakeVector` _relativelocation_x_2 _relativelocation_y_2 _relativelocation_z_2) false false))))))))

(event `self.Box.OnComponentBeginOverlap`
  (params (OverlappedComponent :type "PrimitiveComponent Object Reference") (OtherActor :type "Actor Object Reference") (OtherComp :type "PrimitiveComponent Object Reference") (OtherBodyIndex :type Integer) (bFromSweep :type Boolean) (SweepResult :type "HitResult Structure (by ref)"))
  (if (`self.isOpenDoor`)
    (if (`self.ActorHasTag` OtherActor "Player")
      (`GameplayStatics.OpenLevel` "Demo"))))

(fn `UserConstructionScript`)