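; BP_Murder is an AI killer that hunts the player and jump-scares them on contact.
; A Locomotion/Chase state mirrored to the Blackboard switches to faster Chase when PawnSensing sees the player, reverting on Tick beyond sight radius without resetting speed.
; Overlapping the player plays audio, blends to the face camera, lowers it by timeline, then shows and animates PlayerWB.
; An ActorSpawner all-collect callback, RunToPlayer, briefly disables movement, then restores walking.
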(event `SetState`
  (params (NewState :type "/Game/Blueprints/Murder/E_MurderState Enum" :default "NewEnumerator0"))
  ;[1 1 1] 몬스터 상태 변경
  (if (`|EnumInequality` (`self.State`) NewState)
    (bind _output_get (set `self.State` NewState))
    (`BlackboardComponent.SetValueAsEnum` (`AIBlueprintHelperLibrary.GetBlackboard` (`AIBlueprintHelperLibrary.GetAIController` self)) (`self.StateKey`) _output_get)))

(event `self.ReceiveTick`
  (params (DeltaSeconds :type "Float (single-precision)"))
  (switch `/Game/Blueprints/Murder/E_MurderState` (`self.State`)
    (:`NewEnumerator0`
      (`self.OnLocomotion`))
    (:`NewEnumerator1`
      (`self.OnChase`))))

(event `self.PawnSensing.OnSeePawn`
  (params (Pawn :type "Pawn Object Reference"))
  ;[1 1 1] AI
  (if (`|EnumEquality` (`self.State`) "NewEnumerator0")
    (bind _asbp_player (cast `/Game/Blueprints/BP_Player` Pawn))
    (`self.SetState` "NewEnumerator1")
    (bind _output_get (set `self.Instigator` _asbp_player)) ; 액터가 가지고있는 변수
    (`BlackboardComponent.SetValueAsObject` (`AIBlueprintHelperLibrary.GetBlackboard` (`AIBlueprintHelperLibrary.GetAIController` self)) (`self.TargetPlayerKey`) _output_get)
    (switch `/Game/Blueprints/Murder/E_MurderState` (`self.State`)
      (:`NewEnumerator0`
        (set `CharacterMovementComponent.MaxWalkSpeed` 200.0 (`self.CharacterMovement`)))
      (:`NewEnumerator1`
        (set `CharacterMovementComponent.MaxWalkSpeed` 500.0 (`self.CharacterMovement`))))))

(event `OnLocomotion`)

(event `OnChase`
  (bind _instigator (`self.Instigator`))
  ;[1 1 1] AI Chase Event
  (`/Engine/EditorBlueprintResources/StandardMacros.IsValid` _instigator
    (:`Is Valid`
      (if (> (`KismetMathLibrary.Vector_Distance` (`self.K2_GetActorLocation` _instigator) (`self.K2_GetActorLocation`)) (`PawnSensingComponent.SightRadius` (`self.PawnSensing`)))
        (set `self.Instigator` null)
        (`self.SetState` "NewEnumerator0")))))

(event `self.ReceiveActorBeginOverlap`
  (params (OtherActor :type "Actor Object Reference"))
  (bind _murderfacecamera (`self.MurderFaceCamera`))
  (bind (_relativelocation_x _relativelocation_y) (`KismetMathLibrary.BreakVector` (`SceneComponent.RelativeLocation` _murderfacecamera)))
  (bind _asbp_player (cast `/Game/Blueprints/BP_Player` OtherActor))
  (bind _returnvalue (`AddComponent|NODE_AddAudioComponent-0`))
  (`AudioComponent.Play` _returnvalue 1.0)
  (`PlayerController.SetViewTargetWithBlend` (`PlayerState.GetPlayerController` (`Pawn.PlayerState` _asbp_player)) (`ActorComponent.GetOwner` (`self.MurderFaceCamera`)) 0.325 "VTBlend_Linear" 0.0 false)
  (bind (_direction _jstrack) (`Timeline|타임라인` :!via `PlayFromStart`)
    (:`Update`
      (`SceneComponent.K2_SetRelativeLocation` _murderfacecamera (`KismetMathLibrary.MakeVector` _relativelocation_x _relativelocation_y (`KismetMathLibrary.Lerp` 50.0 35.0 _jstrack)) false false))
    (:`Finished`
      (cast `/Game/Blueprints/BP_Player` (`GameplayStatics.GetPlayerPawn` 0))
      (bind _returnvalue_2 (`|GenericCreateObject` "/Game/Blueprints/Murder/PlayerWB.PlayerWB_C")) ; construct object class
      (`UserWidget.AddToViewport` _returnvalue_2 0)
      (`KismetSystemLibrary.Delay` 3.0)
      (`/Game/Blueprints/Murder/PlayerWB.PlayAnim` _returnvalue_2))))

(event `self.ReceiveBeginPlay`
  (bind _outactors (`GameplayStatics.GetAllActorsOfClass` "/Game/Blueprints/ActorSpawner.ActorSpawner_C"))
  (add `/Game/Blueprints/ActorSpawner.AllCollect` _outactors (delegate `RunToPlayer`)))

(event `RunToPlayer`
  (`CharacterMovementComponent.SetMovementMode` (`self.CharacterMovement`) "MOVE_None" 0)
  (`KismetSystemLibrary.Delay` 4.0)
  (`CharacterMovementComponent.SetMovementMode` (`self.CharacterMovement`) "MOVE_Walking" 0))

(fn `UserConstructionScript`)